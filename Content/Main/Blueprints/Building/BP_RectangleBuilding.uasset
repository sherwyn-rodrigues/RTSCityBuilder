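; A placeable building Blueprint that swaps its own visuals for a turret actor when placed.
; On Onplaced it runs the parent logic, hides its TurretHolder, Turret and Mesh components, and spawns a BP_Turret1 at its location and rotation.
; The turret's AttachActorToActor call keeps world transforms but sets no parent actor.
; The construction script only calls the parent, and a DestroyActor node in the event graph never runs.
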(fn ConstructionScript
  (|CallParentFunction))

(fn Onplaced
  (bind _self self)
  (bind _returnvalue (Transformation|GetActorTransform _self))
  (|CallParentFunction)
  (Rendering|SetVisibility (Variables|Default|GetTurretHolder) false false)
  (bind _returnvalue_2 (Game|SpawnActorfromClass "/Game/Main/Blueprints/Building/BP_Turret1.BP_Turret1_C" (Math|Transform|MakeTransform (.location _returnvalue) (.rotation _returnvalue) "1.000000,1.000000,1.000000") "AdjustIfPossibleButAlwaysSpawn" "MultiplyWithRoot" 0 0))
  (Transformation|AttachActorToActor _returnvalue_2 0 "None" "KeepWorld" "KeepWorld" "KeepWorld" true))