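; Main building actor that tracks its health and takes damage only from actors tagged as enemy AI.
; Each valid hit lowers current health and sends the new health fraction to the health bar on its widget component.
; When health runs out, it clamps to zero, flags the building as dead and hides the health bar, with no destruction logic here.
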(event Game|Damage|EventAnyDamage
  (params (Damage :type Float%20%28single-precision%29) (DamageType :type Damage%20Type%20Object%20Reference) (InstigatedBy :type Controller%20Object%20Reference) (DamageCauser :type Actor%20Object%20Reference))
  (bind _widget (Variables|Default|GetWidget))
  (bind _returnvalue (UserInterface|GetUserWidgetObject _widget))
  (if (Actor|ActorHasTag DamageCauser "EnemyAI")
    (if (> (- (Variables|Default|GetCurrentHealth) Damage) 0.0)
      (bind _output_get (Variables|Default|SetCurrentHealth (- (Variables|Default|GetCurrentHealth) Damage)))
      (Class|BPIHealthBarInterface|UpdateHealth(Message) _returnvalue (/ _output_get (Variables|Default|GetMaxHealth)))
      (else
        (Variables|Default|SetCurrentHealth 0.0)
        (Variables|Default|SetMainBuildingIsDead true)
        (Class|BPIHealthBarInterface|HideHealthBar(Message) _returnvalue)))))

(fn ConstructionScript)