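; BP_Turret1 is a building turret that detects pawns tagged EnemyAI through PawnSensing and fires cannonballs at them.
; On first sighting it locks onto that target and starts looping timers for rotation and firing.
; Rotation eases only the weapon base's yaw toward the target, while firing periodically spawns a CannonBall at the Arrow's transform.
; When the target becomes invalid, both timers clear and tracking resets.
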(event OnSeePawn(PawnSensing)
  (params (Pawn :type Pawn%20Object%20Reference))
  (if (Actor|ActorHasTag Pawn "EnemyAI")
    (Utilities|IsValid Pawn
      (:Is%20Valid
        (if (not (Variables|Default|GetIsTracking))
          (Variables|Default|SetIsTracking true)
          (Variables|Default|SetTargetToTrack Pawn)
          (CallFunction|TrackTarget))))))

(event Custom|Track%20Target
  (bind _returnvalue (Utilities|Time|SetTimerbyEvent (delegate Custom|RotateTurret) 0.05 true true))
  (Variables|Default|SetTimerRefCannonRotate _returnvalue)
  (bind _returnvalue_2 (Utilities|Time|SetTimerbyEvent (delegate Custom|Shoot%20Cannon) 4.0 true true))
  (Variables|Default|SetTimerReferenceCannonShoot _returnvalue_2))

(event Custom|RotateTurret
  (bind _targettotrack (Variables|Default|GetTargetToTrack))
  (bind _weaponbase (Variables|Default|GetWeaponBase))
  (Utilities|IsValid _targettotrack
    (:Is%20Valid
      (Transformation|SetWorldRotation _weaponbase (Math|Rotator|MakeRotator 0.0 0.0 (.yaw (Math|Interpolation|RInterpTo (Transformation|GetWorldRotation _weaponbase) (Math|Rotator|FindLookatRotation (Transformation|GetActorLocation) (Transformation|GetActorLocation _targettotrack)) (Utilities|Time|GetWorldDeltaSeconds) 1e+02))) false false))
    (:Is%20Not%20Valid
      (Utilities|Time|ClearandInvalidateTimerbyHandle (Variables|Default|GetTimerRefCannonRotate))
      (Utilities|Time|ClearandInvalidateTimerbyHandle (Variables|Default|GetTimerReferenceCannonShoot))
      (Variables|Default|SetIsTracking false))))

(event Custom|Shoot%20Cannon
  (if (Variables|Default|GetIsTracking)
    (Game|SpawnActorfromClass "/Game/Main/Blueprints/CannonBall.CannonBall_C" (Transformation|GetWorldTransform (Variables|Default|GetArrow)) "Undefined" "MultiplyWithRoot" 0 0)))

(fn ConstructionScript
  (|CallParentFunction))