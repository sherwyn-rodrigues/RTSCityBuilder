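; City builder game mode that runs endless enemy waves, starting on BeginPlay.
; Each wave spawns twice the wave number in actors at random locations from the first DT_SpawnPoints row.
; EnemyKilled decrements the alive count and, at zero, starts a timer for the next wave.
; The Delay after each spawn sits inside the loop body, so it does not stagger spawns.
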(event Custom|SpawnEnemies
  (Math|Integer|IncrementInt (Variables|Default|GetCurrentWave)
    (:%20%20
      (bind _output_get (Variables|Default|SetMaxEnemiesInCurrentWave (* (Variables|Default|GetCurrentWave) 2)))
      (Variables|Default|SetCurrentEnemiesAlive _output_get)
      (bind _outrownames (DataTable|GetDataTableRowNames "/Game/Main/Blueprints/Data/DT_SpawnPoints.DT_SpawnPoints"))
      (bind _returnvalue (Utilities|GetDataTableRow "/Game/Main/Blueprints/Data/DT_SpawnPoints.DT_SpawnPoints" (Utilities|Array|Get(acopy) _outrownames))
        (:then
          (for _index (range 1 (Variables|Default|GetMaxEnemiesInCurrentWave))
            (if (> (Utilities|Array|Length (.spawnpoints _returnvalue)) 0)
              (Game|SpawnActorfromClass "/Game/Main/Blueprints/AI/BP_EnemyAI.BP_EnemyAI_C" (Math|Transform|MakeTransform (.OutItem (Utilities|Array|Random (.spawnpoints _returnvalue))) "0, 0, 0" "1.000000,1.000000,1.000000") "Undefined" "MultiplyWithRoot" 0 0)
              (Utilities|FlowControl|Delay 1.0)
              (else
                (Development|PrintString "Spawn Points Not Set")))))))))

(event EventBeginPlay
  (CallFunction|SpawnEnemies))

(event EventEnemyKilled
  (bind _result (Math|Integer|DecrementInt (Variables|Default|GetCurrentEnemiesAlive))
    (:%20%20
      (if (== _result 0)
        (Development|PrintString "Level Complete please wiat")
        (Utilities|Time|SetTimerbyEvent (delegate Custom|SpawnEnemies) 5.0)))))

(fn ConstructionScript)