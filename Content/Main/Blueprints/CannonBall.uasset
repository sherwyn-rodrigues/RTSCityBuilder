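; Cannonball projectile that explodes on contact, damaging nearby enemies.
; When its collision component begins an overlap, it spawns an explosion effect and sound at its location.
; A sphere overlap query gathers surrounding pawns and world objects, applies damage only to actors tagged Enemy, then the cannonball destroys itself.
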(event OnComponentBeginOverlap(Collison)
  (params (OverlappedComponent :type Primitive%20Component%20Object%20Reference) (OtherActor :type Actor%20Object%20Reference) (OtherComp :type Primitive%20Component%20Object%20Reference) (OtherBodyIndex :type Integer) (bFromSweep :type Boolean) (SweepResult :type Hit%20Result%20Structure%20%28by%20ref%29))
  (bind _returnvalue (Transformation|GetActorLocation))
  (Effects|SpawnEmitteratLocation "/Game/StarterContent/Particles/P_Explosion.P_Explosion" _returnvalue)
  (Audio|PlaySoundatLocation "/Game/Main/Blueprints/Audio/ExplosionSound.ExplosionSound" _returnvalue "0, 0, 0" 1.0 1.0 0.0 0 0 0 0)
  (bind _outactors (Collision|SphereOverlapActors _returnvalue 2e+02 (Utilities|Array|MakeArray "ObjectTypeQuery3" "ObjectTypeQuery1" "ObjectTypeQuery2") 0 (Utilities|Array|MakeArray self)))
  (for _array_element _outactors
    (if (Actor|ActorHasTag _array_element "Enemy")
      (Game|Damage|ApplyDamage _array_element 1e+01 0 self "/Script/Engine.DamageType")))
  (Actor|DestroyActor))

(fn ConstructionScript)