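; Enemy AI character that melee-attacks nearby actors, intended for the main building, and tracks its own health.
; On BeginPlay it resets the IsCloseToTower blackboard key.
; Attack plays a melee montage, sphere-overlaps at an arrow component, and applies delayed damage to the first hit at half the montage length.
; Incoming damage updates a health bar widget, then flags death and hides the bar at zero health.
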(event Custom|Apply%20damage%20To%20Main%20Building
  (params (DamagedActor :type Actor%20Object%20Reference) (DelayTime :type Float%20%28double-precision%29))
  (Utilities|FlowControl|Delay DelayTime)
  (Game|Damage|ApplyDamage DamagedActor 1e+01 0 self "/Script/Engine.DamageType"))

(event EventBeginPlay
  (bind _self self)
  (bind _returnvalue (AI|GetAIController _self))
  (bind _returnvalue_2 (AI|GetBlackboard _returnvalue))
  (Utilities|IsValid _returnvalue_2
    (:Is%20Valid
      (AI|Components|Blackboard|SetValueasBool _returnvalue_2 (Utilities|Name|MakeLiteralName "IsCloseToTower") false))))

(event Game|Damage|EventAnyDamage
  (params (Damage :type Float%20%28single-precision%29) (DamageType :type Damage%20Type%20Object%20Reference) (InstigatedBy :type Controller%20Object%20Reference) (DamageCauser :type Actor%20Object%20Reference))
  (bind _widget (Variables|Default|GetWidget))
  (bind _returnvalue (UserInterface|GetUserWidgetObject _widget))
  (if (> (- (Variables|Default|GetCurrentEnemyHealth) Damage) 0.0)
    (bind _output_get (Variables|Default|SetCurrentEnemyHealth (- (Variables|Default|GetCurrentEnemyHealth) Damage)))
    (Class|BPIHealthBarInterface|UpdateHealth(Message) _returnvalue (/ _output_get (Variables|Default|GetMaxEnemyHealth)))
    (else
      (Variables|Default|SetCurrentEnemyHealth 0.0)
      (Variables|Default|SetIsDead true)
      (Class|BPIHealthBarInterface|HideHealthBar(Message) _returnvalue))))

(fn ConstructionScript)

(fn Attack
  (bind _returnvalue (Animation|PlayAnimMontage "/Game/Main/Animation/AM_MeeleAttack.AM_MeeleAttack" 1.0 "None"))
  (bind (_outactors _returnvalue_2) (Collision|SphereOverlapActors (Transformation|GetWorldLocation (Variables|Default|GetArrow1)) 1e+02 (Utilities|Array|MakeArray "ObjectTypeQuery1" "ObjectTypeQuery2" "ObjectTypeQuery3") 0 (Utilities|Array|MakeArray self)))
  (if _returnvalue_2
    (for _array_element _outactors
      (CallFunction|ApplyDamagetoMainBuilding _array_element (/ _returnvalue 2.0))
      (return _returnvalue))))