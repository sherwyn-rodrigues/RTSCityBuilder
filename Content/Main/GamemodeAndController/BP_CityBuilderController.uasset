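; City builder player controller that runs camera navigation, building placement and the building-points economy, creating the builder UI and main building on start.
; Enhanced Input pans and zooms the camera pawn, with pan speed scaled by zoom, alongside screen-edge scrolling.
; Placement mode moves a preview actor to the cursor trace; selecting spawns the building if valid, deducts its cost and raises the multiplier.
; A looping timer adds multiplier-scaled points and updates the UI.
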(event Custom|IncreaseBuildingPoints
  (if (Variables|BuildingPoints|GetbIncreasePoints)
    (bind _output_get (Variables|BuildingPoints|SetBuildingPoints (+ (* 1 (Variables|BuildingPoints|GetBuildingPointsMultiplier)) (Variables|BuildingPoints|GetBuildingPoints))))
    (Default|UpdateBuildingPoints (Variables|References|GetPlayerUI) _output_get)))

(event Input|EnhancedActionEvents|EnhancedInputActionIA_MoveFoward
  (params (ActionValue :type Float%20%28double-precision%29) (ElapsedSeconds :type Float%20%28double-precision%29) (TriggeredSeconds :type Float%20%28double-precision%29) (InputAction :type Input%20Action%20Object%20Reference :default "/Game/Main/Input/Actions/IA_MoveFoward.IA_MoveFoward"))
  ;[1 1 1] Movement X
  (if (not (Variables|Default|GetDisableCamNav))
    (Transformation|SetActorTransform (Variables|References|GetCameraPawnRef) (Utilities|MovementX ActionValue (CallFunction|MovementSpeedCalculation) (Variables|Default|GetFastMoveMultiplies) (Variables|References|GetCameraPawnRef)))))

(event Input|EnhancedActionEvents|EnhancedInputActionIA_MoveRight
  (params (ActionValue :type Float%20%28double-precision%29) (ElapsedSeconds :type Float%20%28double-precision%29) (TriggeredSeconds :type Float%20%28double-precision%29) (InputAction :type Input%20Action%20Object%20Reference :default "/Game/Main/Input/Actions/IA_MoveRight.IA_MoveRight"))
  ;[1 1 1] MovementY
  (if (not (Variables|Default|GetDisableCamNav))
    (Transformation|SetActorTransform (Variables|References|GetCameraPawnRef) (Utilities|MovementY ActionValue (CallFunction|MovementSpeedCalculation) (Variables|Default|GetFastMoveMultiplies) (Variables|References|GetCameraPawnRef)))))

(event Input|EnhancedActionEvents|EnhancedInputActionIA_ZoomIn
  (params (ActionValue :type Boolean) (ElapsedSeconds :type Float%20%28double-precision%29) (TriggeredSeconds :type Float%20%28double-precision%29) (InputAction :type Input%20Action%20Object%20Reference :default "/Game/Main/Input/Actions/IA_ZoomIn.IA_ZoomIn"))
  (bind _camerapawnref (Variables|References|GetCameraPawnRef))
  (bind _springarm (Variables|/Game/Main/Blueprints/BP_CameraPawn.BP_CameraPawn_C|GetSpringArm _camerapawnref))
  ;[1 1 1] Zoom in/out
  (Variables|/Script/Engine.SpringArmComponent|SetTargetArmLength _springarm (Math|Float|Clamp(Float) (- (Variables|/Script/Engine.SpringArmComponent|GetTargetArmLength _springarm) (Variables|Default|GetZoomSensetivity)) 1.5e+03 (Variables|Default|GetMaxArmDistance))))

(event Input|EnhancedActionEvents|EnhancedInputActionIA_ZoomOut
  (params (ActionValue :type Boolean) (ElapsedSeconds :type Float%20%28double-precision%29) (TriggeredSeconds :type Float%20%28double-precision%29) (InputAction :type Input%20Action%20Object%20Reference :default "/Game/Main/Input/Actions/IA_ZoomOut.IA_ZoomOut"))
  (bind _camerapawnref (Variables|References|GetCameraPawnRef))
  (bind _springarm (Variables|/Game/Main/Blueprints/BP_CameraPawn.BP_CameraPawn_C|GetSpringArm _camerapawnref))
  ;[1 1 1] Zoom in/out
  (Variables|/Script/Engine.SpringArmComponent|SetTargetArmLength _springarm (Math|Float|Clamp(Float) (+ (Variables|/Script/Engine.SpringArmComponent|GetTargetArmLength _springarm) (Variables|Default|GetZoomSensetivity)) 5e+02 (Variables|Default|GetMaxArmDistance))))

(event Input|EnhancedActionEvents|EnhancedInputActionIA_Select
  (params (ActionValue :type Boolean) (ElapsedSeconds :type Float%20%28double-precision%29) (TriggeredSeconds :type Float%20%28double-precision%29) (InputAction :type Input%20Action%20Object%20Reference :default "/Game/Main/Input/Actions/IA_Select.IA_Select"))
  (if (Variables|Default|GetPlacementModeEnabled)
    (CallFunction|SpawnBuilding)))

(event EventBeginPlay
  (Utilities|FlowControl|Sequence
    (:then_0
      (Input|AddMappingContext (PlayerController|LocalPlayerSubsystems|GetEnhancedInputLocalPlayerSubsystem) "/Game/Main/Input/IMC_Default.IMC_Default" 0 "(bIgnoreAllPressedKeysUntilRelease=True,bForceImmediately=False,bNotifyUserSettings=False)"))
    (:then_1
      (Utilities|ReferenceCasts))
    (:then_2
      (bind _returnvalue (UserInterface|CreateWidget "/Game/Main/UI/WB_BuilderUI.WB_BuilderUI_C"))
      (bind _output_get (Variables|References|SetPlayerUI _returnvalue))
      (UserInterface|Viewport|AddtoViewport _output_get 0)
      (Variables|Default|SetbShowMouseCursor true))
    (:then_3
      (CallFunction|SetPlacementModeEnabled false))
    (:then_4
      (bind _returnvalue_2 (Game|SpawnActorfromClass "/Game/Main/Building/MainBuilding.MainBuilding_C" (Math|Transform|MakeTransform "0.000000,0.000000,-10.000000" "0, 0, 0" "1.000000,1.000000,1.000000") "Undefined" "MultiplyWithRoot" 0 0))
      (Variables|References|SetMainBuildingRef _returnvalue_2))
    (:then_5
      (Utilities|Time|SetTimerbyEvent (delegate Custom|IncreaseBuildingPoints) 1.0 true))))

(event EventTick
  (params (DeltaSeconds :type Float%20%28single-precision%29))
  (if (Variables|Default|GetPlacementModeEnabled)
    (CallFunction|UpdatePlacement)))

(event Input|MouseEvents|MouseX
  (params (AxisValue :type Float%20%28single-precision%29))
  ;[1 1 1] Edge Movement
  (if (not (Variables|Default|GetDisableCamNav))
    (bind (_deltaxspeed _deltayspeed) (Utilities|ScreenEdgeMovement))
    (Transformation|AddActorLocalOffset (Variables|References|GetCameraPawnRef) (Math|Vector|MakeVector _deltaxspeed _deltayspeed 0.0) false false)))

(event Input|MouseEvents|MouseY
  (params (AxisValue :type Float%20%28single-precision%29))
  ;[1 1 1] Edge Movement
  (if (not (Variables|Default|GetDisableCamNav))
    (Utilities|ScreenEdgeMovement) ; enters at MouseY
  ))

(fn ConstructionScript)

(fn MovementSpeedCalculation
  (return (Math|Float|Clamp(Float) (/ (Variables|/Script/Engine.SpringArmComponent|GetTargetArmLength (Variables|/Game/Main/Blueprints/BP_CameraPawn.BP_CameraPawn_C|GetSpringArm (Variables|References|GetCameraPawnRef))) 1e+02) 5.0 2e+01)))

(fn SetPlacementModeEnabled
  (params (IsEnabled :type Boolean))
  (if (== IsEnabled (Variables|Default|GetPlacementModeEnabled))
    (return)
    (else
      (bind _output_get (Variables|Default|SetPlacementModeEnabled IsEnabled))
      (if _output_get
        (bind _returnvalue (Game|SpawnActorfromClass (Variables|References|GetPlaceableActorClass) (Math|Transform|MakeTransform "0.000000,0.000000,-100000.000000") "AlwaysSpawn" "MultiplyWithRoot" 0 0))
        (bind _output_get_2 (Variables|References|SetPlaceableActor _returnvalue))
        (AddComponent|AddBPIsPlaceableComponent _output_get_2)
        (else
          (Utilities|IsValid (Variables|References|GetPlaceableActor)
            (:Is%20Valid
              (Actor|DestroyActor (Variables|References|GetPlaceableActor)))))))))

(fn UpdatePlacement
  (bind _hitresult (Game|Player|GetHitResultUnderCursorbyChannel "TraceTypeQuery3" true))
  (if (.bblockinghit _hitresult)
    (Transformation|SetActorLocation (Variables|References|GetPlaceableActor) (.location _hitresult) false false)))

(fn SpawnBuilding
  (bind _placeableactor (Variables|References|GetPlaceableActor))
  (bind _placeableactor_2 (Variables|References|GetPlaceableActor))
  (bind _returnvalue (Actor|GetComponentbyClass _placeableactor "/Game/Main/Components/BP_IsPlaceableComponent.BP_IsPlaceableComponent_C"))
  (Utilities|IsValid _returnvalue
    (:Is%20Valid
      (if (Variables|/Game/Main/Components/BP_IsPlaceableComponent.BP_IsPlaceableComponent_C|GetIsPlacementValid _returnvalue)
        (Game|SpawnActorfromClass (Variables|References|GetPlaceableActorClass) (Transformation|GetActorTransform _placeableactor_2) "AlwaysSpawn" "MultiplyWithRoot" 0 0)
        (bind _buildingmultiplier (Class|BPIBuildingFunctionInterface|GetBuildingMultiplier(Message) _placeableactor_2))
        (Variables|BuildingPoints|SetBuildingPointsMultiplier (+ _buildingmultiplier (Variables|BuildingPoints|GetBuildingPointsMultiplier)))
        (bind _buildingcost (Class|BPIBuildingFunctionInterface|GetBuildingCost(Message) _placeableactor_2))
        (bind _output_get (Variables|BuildingPoints|SetBuildingPoints (- (Variables|BuildingPoints|GetBuildingPoints) _buildingcost)))
        (Default|UpdateBuildingPoints (Variables|References|GetPlayerUI) _output_get)
        (CallFunction|SetPlacementModeEnabled false)))))

(fn GetBuildingRef
  (return 0))