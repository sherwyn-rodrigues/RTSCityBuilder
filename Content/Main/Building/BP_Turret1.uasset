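; BP_Turret1 is a turret actor that turns to follow an enemy pawn; it contains no firing logic.
; PawnSensing locks onto the first seen pawn tagged EnemyAI and ignores other sightings while tracking.
; A looping timer, rather than Tick, interpolates rotation toward the target, applying only yaw.
; Tracking continues until the target becomes invalid, when the timer clears and the turret can acquire another.
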(event OnSeePawn(PawnSensing)
  (params (Pawn :type Pawn%20Object%20Reference))
  (if (Actor|ActorHasTag Pawn "EnemyAI")
    (Utilities|IsValid Pawn
      (:Is%20Valid
        (if (not (Variables|Default|GetIsTracking))
          (Variables|Default|SetIsTracking true)
          (Variables|Default|SetTargetToTrack Pawn)
          (CallFunction|TrackTarget))))))

(event Custom|Track%20Target
  (bind _returnvalue (Utilities|Time|SetTimerbyEvent (delegate Custom|RotateTurret) 0.05 true))
  (Variables|Default|SetTimerRef _returnvalue))

(event Custom|RotateTurret
  (bind _targettotrack (Variables|Default|GetTargetToTrack))
  (Utilities|IsValid _targettotrack
    (:Is%20Valid
      (Transformation|SetActorRotation (Math|Rotator|MakeRotator 0.0 0.0 (.yaw (Math|Interpolation|RInterpTo (Transformation|GetActorRotation) (Math|Rotator|FindLookatRotation (Transformation|GetActorLocation) (Transformation|GetActorLocation _targettotrack)) (Utilities|Time|GetWorldDeltaSeconds) 1e+02)))))
    (:Is%20Not%20Valid
      (Utilities|Time|ClearandInvalidateTimerbyHandle (Variables|Default|GetTimerRef))
      (Variables|Default|SetIsTracking false))))

(event EventBeginPlay
  (|CallParentFunction) ; This node is disabled and will not be called.\nDrag off pins to build functionality.
)

(event Collision|EventActorBeginOverlap
  (params (OtherActor :type Actor%20Object%20Reference))
  (|CallParentFunction OtherActor) ; This node is disabled and will not be called.\nDrag off pins to build functionality.
)

(event EventTick
  (params (DeltaSeconds :type Float%20%28single-precision%29))
  (|CallParentFunction DeltaSeconds) ; This node is disabled and will not be called.\nDrag off pins to build functionality.
)

(fn ConstructionScript
  (|CallParentFunction))