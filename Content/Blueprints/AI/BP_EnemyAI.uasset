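; Enemy AI character with a melee attack that returns its montage length.
; On BeginPlay it clears the IsCloseToTower blackboard key on its AI controller, printing a warning if the blackboard is invalid.
; Attack starts the melee montage and immediately runs a sphere overlap at Arrow1, without waiting for an anim notify.
; The loop returns after its first hit, so only one overlapped actor takes damage, and a miss never reaches that return.
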(event EventBeginPlay
  (bind _self self)
  (bind _returnvalue (AI|GetAIController _self))
  (bind _returnvalue_2 (AI|GetBlackboard _returnvalue))
  (Utilities|IsValid _returnvalue_2
    (:Is%20Valid
      (AI|Components|Blackboard|SetValueasBool _returnvalue_2 (Utilities|Name|MakeLiteralName "IsCloseToTower") false))
    (:Is%20Not%20Valid
      (Development|PrintString "invalid"))))

(fn ConstructionScript)

(fn Attack
  (bind _returnvalue (Animation|PlayAnimMontage "/Game/Blueprints/Animation/AM_MeeleAttack.AM_MeeleAttack" 1.0 "None"))
  (bind (_outactors _returnvalue_2) (Collision|SphereOverlapActors (Transformation|GetWorldLocation (Variables|Default|GetArrow1)) 1e+02 (Utilities|Array|MakeArray "ObjectTypeQuery1" "ObjectTypeQuery2" "ObjectTypeQuery3") 0 (Utilities|Array|MakeArray self)))
  (if _returnvalue_2
    (for _array_element _outactors
      (Game|Damage|ApplyDamage _array_element 1e+01 0 self "/Script/Engine.DamageType")
      (return _returnvalue))))