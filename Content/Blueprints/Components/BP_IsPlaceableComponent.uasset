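; Actor component that shows whether its owner can be placed, based on whether it overlaps other actors.
; On BeginPlay it binds to the owner's begin and end overlap events and runs an initial check.
; Each check sets IsPlacementValid when no actors overlap, then swaps material slot 0 on all the owner's static meshes to the valid or invalid placement material.
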(event Custom|Overlapped%20status%20changed
  (params (OverlappedActor :type Actor%20Object%20Reference) (OtherActor :type Actor%20Object%20Reference))
  (CallFunction|UpdateMaterial))

(event EventBeginPlay
  (bind _returnvalue (Components|GetOwner))
  (Collision|BindEventtoOnActorBeginOverlap _returnvalue (delegate Custom|Overlapped%20status%20changed))
  (Collision|BindEventtoOnActorEndOverlap _returnvalue (delegate Custom|Overlapped%20status%20changed))
  (CallFunction|UpdateMaterial))

(fn UpdateMaterial
  (bind _output_get (Variables|Default|SetIsPlacementValid (== (Utilities|Array|Length (Collision|GetOverlappingActors (Components|GetOwner) 0 :!class /Script/Engine.Actor)) 0)))
  (for _array_element (Actor|GetComponentsByClass (Components|GetOwner) "/Script/Engine.StaticMeshComponent")
    (if _output_get
      (Rendering|Material|SetMaterial _array_element 0 (Variables|Default|GetValidPlacementMaterial))
      (else
        (Rendering|Material|SetMaterial _array_element 0 (Variables|Default|GetInvalidPlacementMaterial))))))